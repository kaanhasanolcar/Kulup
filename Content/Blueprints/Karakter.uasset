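; Karakter is a player character Blueprint that handles basic keyboard and mouse controls, with Turkish-named input mappings.
; The IleriGeri and SolSag axes move it along the forward and right vectors of the full control rotation, pitch included, and Zipla triggers a jump.
; The SagSolaBak and YukariAsagiBak axes feed controller yaw and pitch for looking around.
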(event Input|ActionEvents|InputActionZipla
  (params (Key :type Key%20Structure :default "AnyKey"))
  ;[1 1 1] Klavye
  (:Pressed
    (Character|Jump)))

(event Input|AxisEvents|InputAxisSagSolaBak
  (params (AxisValue :type Float%20%28single-precision%29))
  ;[1 1 1] Mouse
  (Pawn|Input|AddControllerYawInput AxisValue))

(event Input|AxisEvents|InputAxisYukariAsagiBak
  (params (AxisValue :type Float%20%28single-precision%29))
  ;[1 1 1] Mouse
  (Pawn|Input|AddControllerPitchInput AxisValue))

(event Input|AxisEvents|InputAxisIleriGeri
  (params (AxisValue :type Float%20%28single-precision%29))
  ;[1 1 1] Klavye
  (Pawn|Input|AddMovementInput (Math|Vector|GetForwardVector (Pawn|GetControlRotation :!class /Script/Engine.Pawn)) AxisValue false))

(event Input|AxisEvents|InputAxisSolSag
  (params (AxisValue :type Float%20%28single-precision%29))
  ;[1 1 1] Klavye
  (Pawn|Input|AddMovementInput (Math|Vector|GetRightVector (Pawn|GetControlRotation :!class /Script/Engine.Pawn)) AxisValue false))

(fn ConstructionScript)